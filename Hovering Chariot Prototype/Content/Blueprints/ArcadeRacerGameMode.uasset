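; Game mode for the arcade racer that tracks laps and detects when the race is finished.
; On BeginPlay it creates the racer HUD widget, adds it to the player screen and resets the lap count.
; LapCompleted increments the count, updates the HUD lap counter, then CheckIfWon tells the HUD the game has ended once the count equals the current map's lap amount.
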(event EventBeginPlay
  (Utilities|FlowControl|Sequence
    (:then_0
      (bind _returnvalue (UserInterface|CreateWidget "/Game/Blueprints/ArcadeRacerHUD.ArcadeRacerHUD_C"))
      (bind _output_get (Variables|Default|SetHUD _returnvalue))
      (UserInterface|Viewport|AddtoPlayerScreen _output_get))
    (:then_1
      (Variables|Default|SetLapsCompleted 0))))

(event EventTick
  (params (DeltaSeconds :type Float%20%28single-precision%29)))

(fn ConstructionScript)

(fn CheckifWon
  (if (== (Variables|Default|GetLapAmountCurrentMap) (Variables|Default|GetLapsCompleted))
    (Default|GameEnd (Variables|Default|GetHUD))))

(fn LapCompleted
  (bind _result (Math|Integer|IncrementInt (Variables|Default|GetLapsCompleted))
    (:%20%20
      (bind _output_get (Variables|Default|SetLapsCompleted _result))
      (Default|UpdateLapCounter (Variables|Default|GetHUD) _output_get) ; Update HUD
      (CallFunction|CheckifWon))))