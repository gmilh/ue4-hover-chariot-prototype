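; Player-driven hover vehicle pawn for an arcade racer, with steering, braking, boost and checkpoint respawn.
; Each tick, line traces tilt the Engine component to the terrain normal and drive custom gravity that holds hover height or pulls down increasingly hard when airborne.
; Full forward input on a full meter triggers boost, raising max speed with effects, audio and an FOV timeline while draining the game mode's HUD bar.
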(event Custom|Boost%20Triggered
  (bind _output_get (Variables|Default|SetBoostEngaged true))
  (Components|Activation|SetActive (Variables|Default|GetBoost) _output_get false)
  (Variables|Default|SetCurrent_Boost (Variables|Default|GetMax_Boost))
  (Audio|Components|Audio|Play (Variables|GetFOV))
  (Variables|/Script/Engine.FloatingPawnMovement|SetMaxSpeed (Variables|Default|GetFloatingPawnMovement) (* (Class|MovementComponent|GetMaxSpeed (Variables|Default|GetFloatingPawnMovement)) (Variables|Default|GetBoost_Speed_Multiplier)))
  (Audio|Components|Audio|Stop (Variables|Default|GetBoost%20Audio))
  (Audio|Components|Audio|Play (Variables|Default|GetBoost%20Audio) 0.0)
  (Audio|Components|Audio|Play (Variables|Default|GetFeedbackPlaceholder) 0.0))

(event EventBeginPlay
  ;[0.989 1 0.7298] Initialise Speed
  (Variables|Default|SetCurrent_Speed (Variables|Default|GetDefault_Speed))
  (Variables|Default|SetCurrentCheckpoint (Transformation|GetActorTransform)))

(event EventTick
  (params (DeltaSeconds :type Float%20%28single-precision%29))
  ;[0.3229 1 0.4004] Custom Physics
  (CallFunction|ApplyHovering)
  (CallFunction|ApplyCustomGravity)
  (CallFunction|UpdateBoost))

(event EventPossessed
  (params (NewController :type Controller%20Object%20Reference))
  (Components|Activation|Activate (Variables|Default|GetAudio) false))

(event EventUnpossessed
  (params (OldController :type Controller%20Object%20Reference))
  (Components|Activation|Deactivate (Variables|Default|GetAudio)))

(event Input|AxisEvents|InputAxisMoveRight
  (params (AxisValue :type Float%20%28single-precision%29))
  (bind _returnvalue (Transformation|GetActorRotation))
  ;[0.989 1 0.7298] Vehicle Turning
  (Transformation|SetActorRotation (Math|Rotator|MakeRotator (.roll _returnvalue) (.pitch _returnvalue) (+ (.yaw _returnvalue) AxisValue))))

(event Input|AxisEvents|InputAxisMoveForward
  (params (AxisValue :type Float%20%28single-precision%29))
  (if (Variables|Default|GetBoostEngaged)
    (Pawn|Input|AddMovementInput (Transformation|GetActorForwardVector) (Variables|Default|GetDefault_Speed) false)
    (if (not (Audio|Components|Audio|IsPlaying (Variables|Default|GetBoost%20Audio)))
      (Audio|Components|Audio|Play (Variables|Default|GetBoost%20Audio) 0.0))
    (else
      ;[0.03311 0.402 1] Check if Boosting
      (if (and (>= (Input|AxisValues|GetMoveForward) 0.9) (>= (Variables|Default|GetCurrent_Boost) (Variables|Default|GetMax_Boost)))
        (CallFunction|BoostTriggered)
        (else
          (Variables|Default|SetCurrent_Speed (CallFunction|GetCurrentSpeed))
          (Pawn|Input|AddMovementInput (Transformation|GetActorForwardVector) (Variables|Default|GetCurrent_Speed) false)
          (Audio|Components|Audio|SetPitchMultiplier (Variables|Default|GetAudio) (* 1.5 (Variables|Default|GetCurrent_Speed) (Variables|Default|GetBoost_Speed_Multiplier)))
          (Utilities|String|Reverse (Variables|GetFOV)))))))

(fn ConstructionScript
  (Variables|/Script/Engine.FloatingPawnMovement|SetMaxSpeed (Variables|Default|GetFloatingPawnMovement) (Variables|Default|GetDefault_Speed)))

(fn EmptyBoost
  (Variables|Default|SetCurrent_Boost 0.0))

(fn AddBoost
  (params (Boost%20Collected :type Float%20%28single-precision%29))
  (bind _output_get (Variables|Default|SetCurrent_Boost (select (< (+ Boost%20Collected (Variables|Default|GetCurrent_Boost)) (Variables|Default|GetMax_Boost)) (+ Boost%20Collected (Variables|Default|GetCurrent_Boost)) (Variables|Default|GetMax_Boost))))
  (bind _asarcade_racer_game_mode (Utilities|Casting|CastToArcadeRacerGameMode (Game|GetGameMode)))
  (Default|UpdateBoostBar (Variables|/Game/Blueprints/ArcadeRacerGameMode.ArcadeRacerGameMode_C|GetHUD _asarcade_racer_game_mode) _output_get (Variables|Default|GetMax_Boost))
  (Audio|Components|Audio|Play (Variables|Default|GetFeedbackPlaceholder) 0.0))

(fn RespawnatCheckpoint
  (Transformation|SetActorTransform (Variables|Default|GetCurrentCheckpoint))
  (Variables|/Script/Engine.MovementComponent|SetVelocity (Variables|Default|GetFloatingPawnMovement) "0, 0, 0"))

(fn GetCurrentSpeed
  (bind _returnvalue (Input|AxisValues|GetMoveForward))
  (return (/ (/ (- 1e+02 (* (Math|Float|Absolute(Float) (select (>= _returnvalue 0.0) 0.0 _returnvalue)) (Variables|Default|GetBrake_Percentage))) 1e+02) (Variables|Default|GetBoost_Speed_Multiplier))))

(fn ApplyHovering
  (bind _returnvalue (Transformation|GetActorRotation))
  (bind _engine (Variables|Default|GetEngine))
  (bind _engine_2 (Variables|Default|GetEngine))
  (bind (_x _y) (Math|Rotator|GetAxes _returnvalue))
  ;[1 1 1] Check terrain below front cubes
  (for _array_element (Utilities|Array|MakeArray (Variables|Default|GetStaticMesh4))
    (bind _outhit (Collision|LineTraceByChannel (Transformation|GetWorldLocation _array_element) (+ (Transformation|GetWorldLocation _array_element) (* (Math|Vector|NegateVector (Math|Vector|GetUpVector _array_element)) (Variables|Default|GetTerrainMaxDistance)) (* (Math|Vector|NegateVector (Math|Vector|GetRightVector _array_element)) (Variables|Default|GetTerrainMaxDistance))) "TraceTypeQuery2" false 0 "ForOneFrame"))
    ;[1 1 1] Take the normal from the ground below, then set it as its up vector
    (if (Math|Vector|Equal(Vector) (Variables|Default|GetCurrentTerrainNormal) (.normal _outhit) 0.0)
      (Transformation|SetWorldRotation _engine_2 (Math|Interpolation|RInterpTo (Transformation|GetWorldRotation _engine_2) (Transformation|GetActorRotation) (Utilities|Time|GetWorldDeltaSeconds) 8.9) false false)
      (else
        (Variables|Default|SetCurrentTerrainNormal (.normal _outhit))
        (Transformation|SetWorldRotation _engine (Math|Interpolation|RInterpTo (Transformation|GetWorldRotation _engine) (Math|Rotator|MakeRotationfromAxes _x _y (Variables|Default|GetCurrentTerrainNormal)) (Utilities|Time|GetWorldDeltaSeconds) 4.0) false false)))))

(fn UpdateBoost
  (if (Variables|Default|GetBoostEngaged)
    (bind _output_get (Variables|Default|SetCurrent_Boost (- (Variables|Default|GetCurrent_Boost) (* 1e+02 (Utilities|Time|GetWorldDeltaSeconds)))))
    (bind _asarcade_racer_game_mode (Utilities|Casting|CastToArcadeRacerGameMode (Game|GetGameMode)))
    (Default|UpdateBoostBar (Variables|/Game/Blueprints/ArcadeRacerGameMode.ArcadeRacerGameMode_C|GetHUD _asarcade_racer_game_mode) _output_get (Variables|Default|GetMax_Boost))
    (bind _output_get_2 (Variables|Default|SetBoostEngaged (not (<= (Variables|Default|GetCurrent_Boost) 0.0))))
    (if (not _output_get_2)
      (Variables|Default|SetCurrent_Boost 0.0)
      (Components|Activation|SetActive (Variables|Default|GetBoost) false false)
      (Variables|/Script/Engine.FloatingPawnMovement|SetMaxSpeed (Variables|Default|GetFloatingPawnMovement) (Variables|Default|GetDefault_Speed))
      (Audio|Components|Audio|Stop (Variables|Default|GetBoost%20Audio)))))

(fn ApplyCustomGravity
  (bind _returnvalue (Transformation|GetActorLocation))
  (bind (_outhit _returnvalue_2) (Collision|LineTraceByChannel _returnvalue (+ _returnvalue (* (Math|Vector|NegateVector (Transformation|GetActorUpVector)) (Variables|Default|GetTerrainMaxDistance))) "TraceTypeQuery1" false 0 "None"))
  (if _returnvalue_2
    (Transformation|AddActorLocalOffset (Math|Vector|MakeVector 0.0 0.0 (.z (* (- (+ (.impactpoint _outhit) (Math|Vector|MakeVector 0.0 0.0 (Variables|Default|GetTerrainMaxDistance))) (Transformation|GetActorLocation)) (Utilities|Time|GetWorldDeltaSeconds)))) false true)
    (Variables|Default|SetCurrentGravityPullMultiplier 1.0)
    (else
      (bind _outhit_2 (Collision|LineTraceByChannel (.tracestart _outhit) (+ (.tracestart _outhit) (* (- (.traceend _outhit) (.tracestart _outhit)) 1e+04)) "TraceTypeQuery1" false 0 "None" true "(R=0.136644,G=0.000000,B=1.000000,A=1.000000)"))
      (Transformation|AddActorLocalOffset (Math|Vector|MakeVector 0.0 0.0 (* (Math|Vector|VectorLength (- (.location _outhit_2) (.tracestart _outhit_2))) (Variables|Default|GetGravity%20Base%20Pull) (Utilities|Time|GetWorldDeltaSeconds) -1.0 (Variables|Default|GetCurrentGravityPullMultiplier))) true false)
      (Variables|Default|SetCurrentGravityPullMultiplier (Math|Interpolation|FInterptoConstant (Variables|Default|GetCurrentGravityPullMultiplier) 12.0 (Utilities|Time|GetWorldDeltaSeconds) 1.0)))))