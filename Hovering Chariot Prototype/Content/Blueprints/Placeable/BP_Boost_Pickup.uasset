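; Placeable boost pickup that grants boost to a BP_HoverVehicle that drives into its box trigger.
; On overlap it calls AddBoost with BoostAmount, then plays an explosion particle and pickup sound at its location.
; A DoOnce gates collection while the mesh is deactivated and hidden for CooldownTime, then the mesh returns and the gate resets, so the pickup is reusable.
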(event OnComponentBeginOverlap(Box)
  (params (OverlappedComponent :type Primitive%20Component%20Object%20Reference) (OtherActor :type Actor%20Object%20Reference) (OtherComp :type Primitive%20Component%20Object%20Reference) (OtherBodyIndex :type Integer) (bFromSweep :type Boolean) (SweepResult :type Hit%20Result%20Structure%20%28by%20ref%29))
  (bind _returnvalue (Transformation|GetActorLocation))
  ;[1 1 1] When Overlapping with player, increase boost
  (bind _asbp_hover_vehicle (Utilities|Casting|CastToBP_HoverVehicle OtherActor))
  (Utilities|FlowControl|DoOnce false :!label _label
    (:Completed
      (Default|AddBoost _asbp_hover_vehicle (Variables|Default|GetBoostAmount))
      (Effects|SpawnEmitteratLocation "/Game/Particles/P_Explosion.P_Explosion" _returnvalue)
      (Audio|PlaySoundatLocation "/Game/Sounds/metal_pickup.metal_pickup" _returnvalue)
      ;[1 1 1] Deactivate pickup on collection, cooldown and reactivate
      (Components|Activation|Deactivate (Variables|Default|GetStaticMesh))
      (Rendering|SetVisibility (Variables|Default|GetStaticMesh) false false)
      (Utilities|FlowControl|Delay (Variables|Default|GetCooldown%20Time))
      (Components|Activation|Activate (Variables|Default|GetStaticMesh) false)
      (Rendering|SetVisibility (Variables|Default|GetStaticMesh) true false)
      (goto _label Reset))))

(event EventBeginPlay)

(event Collision|EventActorBeginOverlap
  (params (OtherActor :type Actor%20Object%20Reference)))

(event EventTick
  (params (DeltaSeconds :type Float%20%28single-precision%29)))

(fn ConstructionScript)